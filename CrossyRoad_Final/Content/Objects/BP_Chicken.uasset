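; BP_Chicken is the player chicken in a Crossy Road-style game, hopping one tile per input and scoring forward progress.
; A Move timeline lerps each hop with input disabled, snapping to the grid except on logs, while MovableLeft/Right limit sideways moves.
; Tick flattens the chicken on vehicle, drowning or eagle death, spawns a one-time effect and blends to the death camera.
; Leaving the Y bounds also moves the camera, but DeathOutsidePlayzone stays false.
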(event Custom|MoveToTile
  (bind _current_pos (Variables|Default|Getcurrent%20pos))
  ;[1 1 1] Move process ( 1 tile at the time)
  (bind _moveprocess (Timeline|Move PlayFromStart)
    (:Update
      (Transformation|SetActorLocation (Math|Vector|Lerp(Vector) (Variables|Default|Getcurrent%20pos) (Math|Vector|MakeVector (select (Variables|Default|Geton%20log) (+ (* (Variables|Default|Getup) 1e+02) (.x _current_pos)) (+ (* (Variables|Default|Getup) 1e+02) (* (Math|Float|Round (/ (.x _current_pos) 1e+02)) 1e+02))) (select (Variables|Default|Geton%20log) (+ (* (Variables|Default|Getright) 8e+01) (.y _current_pos)) (+ (* (Variables|Default|Getright) 1e+02) (* (Math|Float|Round (/ (.y _current_pos) 1e+02)) 1e+02))) (select (<= _moveprocess 0.6) (Variables|Default|Getjump%20height) (- (Variables|Default|Getjump%20height) 135.0))) _moveprocess) true false))
    (:Finished
      (Input|EnableInput 0)
      (if (> (Math|Float|Round (/ (+ (.x (Transformation|GetActorLocation)) 9e+01) 1e+02)) (Variables|Default|Getscore))
        (Variables|Default|Setscore (+ (Variables|Default|Getscore) 1))))))

(event EventBeginPlay
  ;[1 1 1] death effect
  (Variables|Default|Seteffect false))

(event EventTick
  (params (DeltaSeconds :type Float%20%28single-precision%29))
  (bind _returnvalue (Transformation|GetActorLocation))
  ;[1 1 1] death effect
  (if (Variables|Default|Getdeath%20by%20vehicle)
    (Transformation|SetActorTransform (Math|Transform|MakeTransform (Math|Vector|MakeVector (.x (Variables|Default|Getcurrent%20pos)) (.y (Variables|Default|Getcurrent%20pos)) 0.1) "0, 0, 0" "1,1,0.001000"))
    (if (not (Variables|Default|Geteffect))
      (Game|SpawnActorfromClass "/Game/Meshes/BP_Feather.BP_Feather_C" (Math|Transform|MakeTransform (Math|Vector|MakeVector (.x (Variables|Default|Getcurrent%20pos)) (.y (Variables|Default|Getcurrent%20pos)) (.z (Variables|Default|Getcurrent%20pos))) "0, 0, 0" "1,1,1") "Undefined" 0 0)
      (Variables|Default|Seteffect true)
      (Transformation|SetWorldLocation (Variables|Default|GetCamera) (Math|Vector|MakeVector (.x (Variables|Default|Getcurrent%20pos)) (- (.y (Variables|Default|Getcurrent%20pos)) -3e+02) 2.1e+02) false false)
      (Game|Player|SetViewTargetwithBlend (Game|GetPlayerController 0) (Components|GetOwner (Variables|Default|GetCamera)) 2.0 "VTBlend_Linear" 0.0 false))
    (elif (Variables|Default|Getdeath%20by%20drowning)
      (Transformation|SetActorTransform (Math|Transform|MakeTransform (Math|Vector|MakeVector (.x (Variables|Default|Getcurrent%20pos)) (.y (Variables|Default|Getcurrent%20pos)) 5.0) "0, 0, 0" "1,1,0.100000"))
      (if (not (Variables|Default|Geteffect))
        (Game|SpawnActorfromClass "/Game/Meshes/BP_Water_splash.BP_Water_splash_C" (Math|Transform|MakeTransform (Math|Vector|MakeVector (.x (Variables|Default|Getcurrent%20pos)) (.y (Variables|Default|Getcurrent%20pos)) (.z (Variables|Default|Getcurrent%20pos))) "0, 0, 0" "1,1,1") "Undefined" 0 0)
        (Variables|Default|Seteffect true)
        (Transformation|SetWorldLocation (Variables|Default|GetCamera) (Math|Vector|MakeVector (.x (Variables|Default|Getcurrent%20pos)) (+ (.y (Variables|Default|Getcurrent%20pos)) 4e+02) 2e+02) false false)
        (Game|Player|SetViewTargetwithBlend (Game|GetPlayerController 0) (Components|GetOwner (Variables|Default|GetCamera)) 2.0 "VTBlend_Linear" 0.0 false))
      (elif (Variables|Default|Getdeath%20by%20eagle)
        (Transformation|SetActorTransform (Math|Transform|MakeTransform (Math|Vector|MakeVector (.x (Variables|Default|Getcurrent%20pos)) (.y (Variables|Default|Getcurrent%20pos)) 0.0) "0, 0, 0" "1,1,0.100000"))
        (if (not (Variables|Default|Geteffect))
          (Game|SpawnActorfromClass "/Game/Meshes/BP_Feather.BP_Feather_C" (Math|Transform|MakeTransform (Math|Vector|MakeVector (.x (Variables|Default|Getcurrent%20pos)) (.y (Variables|Default|Getcurrent%20pos)) (.z (Variables|Default|Getcurrent%20pos))) "0, 0, 0" "1,1,1") "Undefined" 0 0)
          (Variables|Default|Seteffect true)
          (Transformation|SetWorldLocation (Variables|Default|GetCamera) (Math|Vector|MakeVector (.x (Variables|Default|Getcurrent%20pos)) (+ (.y (Variables|Default|Getcurrent%20pos)) 4e+02) 2.1e+02) false false)
          (Game|Player|SetViewTargetwithBlend (Game|GetPlayerController 0) (Components|GetOwner (Variables|Default|GetCamera)) 2.0 "VTBlend_Linear" 0.0 false))
        (elif (not (Variables|Default|Getdeath%20outside%20playzone))
          (if (or (< (.y _returnvalue) 4e+02) (> (.y _returnvalue) 2.5e+03))
            (Variables|Default|Setdeath%20outside%20playzone false)
            (Variables|Default|Setcurrent%20pos (Transformation|GetActorLocation))
            (Transformation|SetActorLocation (Math|Vector|MakeVector (.x (Variables|Default|Getcurrent%20pos)) (.y (Variables|Default|Getcurrent%20pos)) 0.0) false false)
            (Transformation|SetWorldLocation (Variables|Default|GetCamera) (Math|Vector|MakeVector (.x (Variables|Default|Getcurrent%20pos)) (+ (.y (Variables|Default|Getcurrent%20pos)) 4e+02) 2e+02) false false)
            (Game|Player|SetViewTargetwithBlend (Game|GetPlayerController 0) (Components|GetOwner (Variables|Default|GetCamera)) 2.0 "VTBlend_Linear" 0.0 false)))))))

(event Input|ActionEvents|InputActionMoveRight
  (params (Key :type Key%20Structure :default "None"))
  ;[1 1 1] Chicken movement
  (:Pressed
    (bind _movable (CallFunction|MovableRight (Utilities|Struct|MakeCoordinate 0 (Math|Float|Round (/ (.y (Transformation|GetActorLocation)) 1e+02)))))
    (if _movable
      (Input|DisableInput 0)
      (if (not (Math|Boolean|ORBoolean (Variables|Default|Getdeath%20by%20vehicle) (Variables|Default|Getdeath%20by%20drowning) (Variables|Default|Getdeath%20by%20eagle) (Variables|Default|Getdeath%20outside%20playzone)))
        (Variables|Default|Setcurrent%20pos (Transformation|GetActorLocation))
        (Variables|Default|Setup 0.0)
        (Variables|Default|Setright 1.0)
        (Transformation|SetWorldRotation (Variables|Character|GetMesh) "0,90.000000, 0" false false)
        (CallFunction|MovetoTile)))))

(event Input|ActionEvents|InputActionMoverForward
  (params (Key :type Key%20Structure :default "None"))
  ;[1 1 1] Chicken movement
  (:Pressed
    (Input|DisableInput 0)
    (if (not (Math|Boolean|ORBoolean (Variables|Default|Getdeath%20by%20vehicle) (Variables|Default|Getdeath%20by%20drowning) (Variables|Default|Getdeath%20by%20eagle) (Variables|Default|Getdeath%20outside%20playzone)))
      (Variables|Default|Setcurrent%20pos (Transformation|GetActorLocation))
      (Variables|Default|Setup 1.0)
      (Variables|Default|Setright 0.0)
      (Transformation|SetWorldRotation (Variables|Character|GetMesh) "0, 0, 0" false false)
      (CallFunction|MovetoTile))))

(event Input|ActionEvents|InputActionMoveBackward
  (params (Key :type Key%20Structure :default "None"))
  ;[1 1 1] Chicken movement
  (:Pressed
    (Input|DisableInput 0)
    (if (not (Math|Boolean|ORBoolean (Variables|Default|Getdeath%20by%20vehicle) (Variables|Default|Getdeath%20by%20drowning) (Variables|Default|Getdeath%20by%20eagle) (Variables|Default|Getdeath%20outside%20playzone)))
      (Variables|Default|Setcurrent%20pos (Transformation|GetActorLocation))
      (Variables|Default|Setup -1.0)
      (Variables|Default|Setright 0.0)
      (Transformation|SetWorldRotation (Variables|Character|GetMesh) "0,180.000000, 0" false false)
      (CallFunction|MovetoTile))))

(event Input|ActionEvents|InputActionMoveLeft
  (params (Key :type Key%20Structure :default "None"))
  ;[1 1 1] Chicken movement
  (:Pressed
    (bind _movable (CallFunction|MovableLeft (Utilities|Struct|MakeCoordinate 0 (Math|Float|Round (/ (.y (Transformation|GetActorLocation)) 1e+02)))))
    (if _movable
      (Input|DisableInput 0)
      (if (not (Math|Boolean|ORBoolean (Variables|Default|Getdeath%20by%20vehicle) (Variables|Default|Getdeath%20by%20drowning) (Variables|Default|Getdeath%20by%20eagle) (Variables|Default|Getdeath%20outside%20playzone)))
        (Variables|Default|Setcurrent%20pos (Transformation|GetActorLocation))
        (Variables|Default|Setup 0.0)
        (Variables|Default|Setright -1.0)
        (Transformation|SetWorldRotation (Variables|Character|GetMesh) "0,-90.000000, 0" false false)
        (CallFunction|MovetoTile)))))

(fn ConstructionScript)

(fn MovableLeft
  (params (coord :type Coordinate%20Structure))
  (if (> (.y coord) 7)
    (return true)
    (else
      (return false))))

(fn MovableRight
  (params (coord :type Coordinate%20Structure))
  (if (< (.y coord) (- (Variables|Default|Getwidth) 8))
    (return true)
    (else
      (return false))))