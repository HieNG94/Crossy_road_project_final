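; Moving wooden log hazard-crossing platform that the chicken can ride, in what appears to be a Frogger-style game.
; Tick sweeps the log along its local X axis at LogSpeed and destroys it once it leaves a world Y range.
; Box overlap flags a chicken that is neither drowned nor on a leaf as OnLog and sets the log's own height to a fixed Z.
; End overlap clears that flag.
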(event OnComponentBeginOverlap(Box)
  (params (OverlappedComponent :type Primitive%20Component%20Object%20Reference) (OtherActor :type Actor%20Object%20Reference) (OtherComp :type Primitive%20Component%20Object%20Reference) (OtherBodyIndex :type Integer) (bFromSweep :type Boolean) (SweepResult :type Hit%20Result%20Structure%20%28by%20ref%29))
  (bind _returnvalue (Transformation|GetActorLocation))
  (bind _asbp_chicken (Utilities|Casting|CastToBP_Chicken OtherActor))
  (if (not (Variables|/Game/Objects/BP_Chicken.BP_Chicken_C|Getdeath%20by%20drowning _asbp_chicken))
    (if (not (Variables|/Game/Objects/BP_Chicken.BP_Chicken_C|Geton%20leaf _asbp_chicken))
      (Variables|/Game/Objects/BP_Chicken.BP_Chicken_C|Seton%20log _asbp_chicken true)
      (Transformation|SetActorLocation (Math|Vector|MakeVector (.x _returnvalue) (.y _returnvalue) 6.0) false false))))

(event OnComponentEndOverlap(Box)
  (params (OverlappedComponent :type Primitive%20Component%20Object%20Reference) (OtherActor :type Actor%20Object%20Reference) (OtherComp :type Primitive%20Component%20Object%20Reference) (OtherBodyIndex :type Integer))
  (bind _asbp_chicken (Utilities|Casting|CastToBP_Chicken OtherActor))
  (Variables|/Game/Objects/BP_Chicken.BP_Chicken_C|Seton%20log _asbp_chicken false))

(event EventTick
  (params (DeltaSeconds :type Float%20%28single-precision%29))
  (Transformation|AddActorLocalOffset (Math|Vector|MakeVector (* DeltaSeconds (Variables|Default|Getlog%20speed)) 0.0 0.0) true false)
  (if (or (> (.y (Transformation|GetActorLocation self)) 3.2e+03) (< (.y (Transformation|GetActorLocation self)) -5e+02))
    (Actor|DestroyActor self)))

(fn ConstructionScript)